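; A display actor that shows a character's armor-blasting damage render targets on three quads: damage, time damage and time-damage backup.
; BeginPlay gives each quad mesh its own dynamic material instance.
; Tick polls the Character's Blastable component until all three render targets are valid, binds each to its quad's RT_Damage texture parameter, then disables ticking.
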(event EventBeginPlay
  (bind _staticmeshcomponent (Variables|Debug|GetStaticMeshComponent))
  (bind _temporaldamagedisplay (Variables|Default|GetTemporalDamageDisplay))
  (bind _temporaldamagebackupdisplay (Variables|Default|GetTemporalDamageBackupDisplay))
  ;[1 1 1] Initialize dynamic material instance for each quad
  (bind _returnvalue (Rendering|Material|CreateDynamicMaterialInstance (Rendering|Material|GetMaterial _staticmeshcomponent 0) "None" :!class /Script/Engine.KismetMaterialLibrary))
  (Rendering|Material|SetMaterial _staticmeshcomponent 0 _returnvalue)
  (bind _returnvalue_2 (Rendering|Material|CreateDynamicMaterialInstance (Rendering|Material|GetMaterial _temporaldamagedisplay 0) "None" :!class /Script/Engine.KismetMaterialLibrary))
  (Rendering|Material|SetMaterial _temporaldamagedisplay 0 _returnvalue_2)
  (bind _returnvalue_3 (Rendering|Material|CreateDynamicMaterialInstance (Rendering|Material|GetMaterial _temporaldamagebackupdisplay 0) "None" :!class /Script/Engine.KismetMaterialLibrary))
  (Rendering|Material|SetMaterial _temporaldamagebackupdisplay 0 _returnvalue_3))

(event Collision|EventActorBeginOverlap
  (params (OtherActor :type Actor%20Object%20Reference)))

(event EventTick
  (params (DeltaSeconds :type Float%20%28single-precision%29))
  (bind _character (Variables|Default|GetCharacter))
  (bind _returnvalue (Class|BlastableCharacter|GetBlastableComponent _character))
  (bind _returnvalue_2 (Class|BlastableComponent|GetTimeDamageBackupRenderTarget _returnvalue))
  (bind _returnvalue_3 (Class|BlastableComponent|GetDamageRenderTarget _returnvalue))
  (bind _returnvalue_4 (Class|BlastableComponent|GetTimeDamageRenderTarget _returnvalue))
  (Variables|Default|SetDamageRenderTarget _returnvalue_3)
  (Variables|Default|SetTimeDamageRenderTarget _returnvalue_4)
  (Variables|Default|SetTimeDamageBackupRenderTarget _returnvalue_2)
  (if (and (and (Utilities|IsValid _returnvalue_3) (Utilities|IsValid _returnvalue_4)) (Utilities|IsValid _returnvalue_2))
    (CallFunction|SetRenderTarget (Variables|Default|GetDamageRenderTarget) (Variables|Default|GetTimeDamageRenderTarget) (Variables|Default|GetTimeDamageBackupRenderTarget))
    (Actor|Tick|SetActorTickEnabled self)))

(fn ConstructionScript)

(fn SetRenderTarget
  (params (DamageRenderTarget :type Texture%20Object%20Reference) (TimeDamageRenderTarget :type Texture%20Object%20Reference) (TimeDamageBackupRenderTarget :type Texture%20Object%20Reference))
  (bind _asmaterial_instance_dynamic (Utilities|Casting|CastToMaterialInstanceDynamic (Rendering|Material|GetMaterial (Variables|Debug|GetStaticMeshComponent) 0)))
  (Rendering|Material|SetTextureParameterValue _asmaterial_instance_dynamic "RT_Damage" DamageRenderTarget)
  (bind _asmaterial_instance_dynamic_2 (Utilities|Casting|CastToMaterialInstanceDynamic (Rendering|Material|GetMaterial (Variables|Default|GetTemporalDamageDisplay) 0)))
  (Rendering|Material|SetTextureParameterValue _asmaterial_instance_dynamic_2 "RT_Damage" TimeDamageRenderTarget)
  (bind _asmaterial_instance_dynamic_3 (Utilities|Casting|CastToMaterialInstanceDynamic (Rendering|Material|GetMaterial (Variables|Default|GetTemporalDamageBackupDisplay) 0)))
  (Rendering|Material|SetTextureParameterValue _asmaterial_instance_dynamic_3 "RT_Damage" TimeDamageBackupRenderTarget))